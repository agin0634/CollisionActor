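; BP_CollisionActorComponent is an actor component that attaches collision part actors to sockets on its owner's skeletal mesh.
; On BeginPlay in Skeleton Mesh mode, it spawns a BP_CollisionActorPart for each CollisionData entry at the socket transform plus offset.
; Each part attaches to its socket and receives that entry's data, including particle settings.
; A missing mesh or socket prints an error; static mesh hit binding is unconnected.
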(event Custom|Hit
  (params (HitComponent :type Primitive%20Component%20Object%20Reference) (OtherActor :type Actor%20Object%20Reference) (OtherComp :type Primitive%20Component%20Object%20Reference) (NormalImpulse :type Vector) (Hit :type Hit%20Result%20Structure%20%28by%20ref%29)))

(event EventBeginPlay
  (bind _returnvalue (Components|GetOwner))
  (bind _returnvalue_2 (Actor|GetComponentbyClass _returnvalue "/Script/Engine.SkeletalMeshComponent"))
  (switch Utilities|FlowControl|Switch|SwitchonEOwnerType (Variables|OwnerDefault|GetType)
    (:NewEnumerator0
      ;[1 1 1] Skeleton Mesh
      (Utilities|IsValid _returnvalue_2
        (:Is%20Valid
          (Variables|OwnerDefault|SetOwner _returnvalue_2)
          (for _array_element (Variables|CollisionData|GetCollisionData)
            (CallFunction|SpawnCollisionActor _array_element)))
        (:Is%20Not%20Valid
          (Development|PrintString "No Skeleton Mesh found" true true "(R=1.000000,G=0.055564,B=0.000000,A=1.000000)"))))))

(event EventTick
  (params (DeltaSeconds :type Float%20%28single-precision%29)))

(fn SpawnCollisionActor
  (params (CollisionData :type Collision%20Actor%20Data%20Structure))
  (bind _owner (Variables|OwnerDefault|GetOwner))
  (Utilities|FlowControl|Sequence
    (:then_0
      ;[1 1 1] Setup Local Variables
      (LocalVariables|SetSocketName (.socketname CollisionData))
      (LocalVariables|SetOffset (.offset CollisionData))
      (LocalVariables|SetbActivateParticle (.activateparticle CollisionData))
      (LocalVariables|SetTemplate (.particletemplate CollisionData))
      (LocalVariables|SetGap (.gap CollisionData)))
    (:then_1
      (if (Transformation|DoesSocketExist _owner (LocalVariables|GetSocketName))
        (bind _returnvalue (Game|SpawnActorfromClass "/Game/CollisionActor/BP_CollisionActorPart.BP_CollisionActorPart_C" (Math|Transform|MakeTransform (+ (.location (Transformation|GetSocketTransform _owner (LocalVariables|GetSocketName) "RTS_World")) (.Location (Math|Transform|BreakTransform (LocalVariables|GetOffset)))) (Math|Rotator|MakeRotator (+ (.Roll (Math|Rotator|BreakRotator (.rotation (Transformation|GetSocketTransform _owner (LocalVariables|GetSocketName) "RTS_World")))) (.Roll (Math|Rotator|BreakRotator (.Rotation (Math|Transform|BreakTransform (LocalVariables|GetOffset)))))) (+ (.Pitch (Math|Rotator|BreakRotator (.rotation (Transformation|GetSocketTransform _owner (LocalVariables|GetSocketName) "RTS_World")))) (.Pitch (Math|Rotator|BreakRotator (.Rotation (Math|Transform|BreakTransform (LocalVariables|GetOffset)))))) (+ (.Yaw (Math|Rotator|BreakRotator (.rotation (Transformation|GetSocketTransform _owner (LocalVariables|GetSocketName) "RTS_World")))) (.Yaw (Math|Rotator|BreakRotator (.Rotation (Math|Transform|BreakTransform (LocalVariables|GetOffset))))))) (* (.scale (Transformation|GetSocketTransform _owner (LocalVariables|GetSocketName) "RTS_World")) (.Scale (Math|Transform|BreakTransform (LocalVariables|GetOffset))))) "Undefined" 0 0))
        (Transformation|AttachComponentToComponent _returnvalue (Variables|OwnerDefault|GetOwner) (LocalVariables|GetSocketName) "KeepWorld" "KeepWorld" "KeepWorld" true)
        (Variables|/Game/CollisionActor/BP_CollisionActorPart.BP_CollisionActorPart_C|SetData _returnvalue (Utilities|Struct|MakeCollisionActorData (LocalVariables|GetSocketName) (LocalVariables|GetOffset) (LocalVariables|GetbActivateParticle) (LocalVariables|GetTemplate) (LocalVariables|GetGap)))
        (else
          (Development|PrintString "No Socket Name found" true true "(R=1.000000,G=0.026892,B=0.000000,A=1.000000)"))))))