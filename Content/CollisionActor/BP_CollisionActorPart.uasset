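; BP_CollisionActorPart is a collision sphere actor that emits particles as it moves while overlapping something.
; Sphere begin and end overlaps open and close a gate on Tick, which calls ActivateParticle while open.
; When enabled in Data, that function spawns the template attached to the root if movement since the last check reaches Data.Gap.
; It then stores the current location either way, so Gap acts as a per-tick movement threshold.
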(event OnComponentBeginOverlap(Sphere)
  (params (OverlappedComponent :type Primitive%20Component%20Object%20Reference) (OtherActor :type Actor%20Object%20Reference) (OtherComp :type Primitive%20Component%20Object%20Reference) (OtherBodyIndex :type Integer) (bFromSweep :type Boolean) (SweepResult :type Hit%20Result%20Structure%20%28by%20ref%29))
  (Utilities|FlowControl|Gate true) ; enters at Open
)

(event OnComponentEndOverlap(Sphere)
  (params (OverlappedComponent :type Primitive%20Component%20Object%20Reference) (OtherActor :type Actor%20Object%20Reference) (OtherComp :type Primitive%20Component%20Object%20Reference) (OtherBodyIndex :type Integer))
  (Utilities|FlowControl|Gate true) ; enters at Close
)

(event EventBeginPlay
  (Variables|Default|SetPreviousLocation (Transformation|GetWorldLocation (Variables|Default|GetSphere))))

(event EventTick
  (params (DeltaSeconds :type Float%20%28single-precision%29))
  (Variables|Default|SetCurrentLocation (Transformation|GetWorldLocation (Variables|Default|GetSphere)))
  (Utilities|FlowControl|Gate true
    (:Exit
      (CallFunction|ActivateParticle))))

(fn ConstructionScript)

(fn ActivateParticle
  (bind _data (Variables|Default|GetData))
  (if (.activateparticle _data)
    (Utilities|IsValid (.particletemplate _data)
      (:Is%20Valid
        (if (>= (Math|Vector|Distance(Vector) (Variables|Default|GetCurrentLocation) (Variables|Default|GetPreviousLocation)) (.gap _data))
          (Effects|SpawnEmitterAttached (.particletemplate _data) (Variables|Default|GetDefaultSceneRoot) "None" "0, 0, 0" "0, 0, 0" "1.000000,1.000000,1.000000" "SnapToTarget"))
        (Variables|Default|SetPreviousLocation (Variables|Default|GetCurrentLocation)))
      (:Is%20Not%20Valid
        (Development|PrintString "No Particle Template found")))))